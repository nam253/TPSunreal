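; Enemy state machine component for BP_Enemy that targets BP_TPSPlayer through Idle, Move, Attack, Damage and Die states.
; Tick dispatches by state using a shared delay timer, but calls the attack animation every frame regardless of state.
; Move steers toward the player until in range; Attack only rechecks range, and Damage returns to Idle immediately, ignoring its timer.
; OnDamageProcess decrements HP; death disables capsule collision and sinks the enemy until destroyed.
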(event `self.ReceiveBeginPlay`
  (bind _returnvalue (`GameplayStatics.GetActorOfClass` "/Game/Blueprint/BP_TPSPlayer.BP_TPSPlayer_C"))
  ; Me가 BP_Enemy인 것을 알 수 있도록 소유 객체를 가져온다.
  (set `self.Target` _returnvalue)
  (bind _asbp_enemy (cast `/Game/Blueprint/BP_Enemy` (`self.GetOwner`)))
  (bind _output_get (set `self.Me` _asbp_enemy))
  (bind _asabp_enemy (cast `/Game/Blueprint/ABP_Enemy` (`SkeletalMeshComponent.GetAnimInstance` (`Character.Mesh` _output_get))))
  (set `self.Anim` _asabp_enemy))

(event `self.ReceiveTick`
  (params (DeltaSeconds :type "Float (single-precision)"))
  (bind _enemystate (`self.EnemyState`))
  (`KismetSystemLibrary.PrintString` (`|GetEnumeratorNameAsString` _enemystate) true false)
  (`/Game/Blueprint/ABP_Enemy.PlayAttackAnim` (`self.Anim`))
  (switch `/Game/Blueprint/E_EnemyState` _enemystate
    (:`NewEnumerator0`
      (`self.IdleState`))
    (:`NewEnumerator1`
      (`self.MoveState`))
    (:`NewEnumerator2`
      (`self.AttackState`))
    (:`NewEnumerator3`
      (`self.DamageState`))
    (:`NewEnumerator4`
      (`self.DieState`))))

(fn `AttackState`
  (bind _isfinish_ (`self.Time Flow` (`self.AttackDelayTime`)))
  (if _isfinish_
    ; 타겟이 공격 범위를 벗어나면 이동(Move State)로 전환
    (if (> (`KismetMathLibrary.Vector_Distance` (`Actor.K2_GetActorLocation` (`self.Target`)) (`Actor.K2_GetActorLocation` (`self.Me`))) (`self.AttackRange`))
      (set `self.EnemyState` "NewEnumerator1"))))

(fn `DamageState`
  (`self.Time Flow` (`self.DamageDelayTime`))
  (if true
    (set `self.EnemyState` "NewEnumerator0")))

(fn `DieState`
  (bind (_returnvalue_x _returnvalue_y _returnvalue_z) (`KismetMathLibrary.BreakVector` (`Actor.K2_GetActorLocation` (`self.Me`))))
  (`Actor.K2_SetActorLocation` (`self.Me`) (+ (`Actor.K2_GetActorLocation` (`self.Me`)) (* (* (`KismetMathLibrary.Vector_Down`) (`self.DieSpeed`)) (`GameplayStatics.GetWorldDeltaSeconds`))) false false)
  (if (< _returnvalue_z -200.0)
    (`Actor.K2_DestroyActor` (`self.Me`))))

(fn `IdleState`
  ; 경과 시간이 대기시간을 초과했다면
  (bind _isfinish_ (`self.Time Flow` (`self.IdleDelayTime`)))
  (if _isfinish_
    ; 이동 상태로 전환하고 싶다.
    (set `self.EnemyState` "NewEnumerator1")))

(fn `MoveState`
  (locals (Direction :type "Vector Structure") (Distance :type "Float (double-precision)"))
  (bind _returnvalue (- (`Actor.K2_GetActorLocation` (`self.Target`)) (`Actor.K2_GetActorLocation` (`self.Me`))))
  (set `local.Distance` (`KismetMathLibrary.VSize` _returnvalue))
  (bind _output_get (set `local.Direction` (`KismetMathLibrary.Normal` _returnvalue)))
  (`Pawn.AddMovementInput` (`self.Me`) _output_get 1.0 false)
  ; 타겟이 일정 범위내로 들어오면 공격 상태로 전환
  (if (< (`local.Distance`) (`self.AttackRange`))
    (set `self.EnemyState` "NewEnumerator2")
    (set `self.CurrentTime` (`self.AttackDelayTime`))))

(fn `OnDamageProcess`
  (set `self.CurrentTime` 0.0)
  (bind _result (`/Engine/EditorBlueprintResources/StandardMacros.DecrementInt` (`self.HP`))
    (:`  `
      (if (> _result 0)
        (set `self.EnemyState` "NewEnumerator3")
        (else
          (set `self.EnemyState` "NewEnumerator4")
          (`PrimitiveComponent.SetCollisionEnabled` (`Character.CapsuleComponent` (`self.Me`)) "NoCollision"))))))

(fn `Time Flow`
  (params (DelayTime :type "Float (double-precision)"))
  (returns (`IsFinish?` :type Boolean))
  (bind _output_get (set `self.CurrentTime` (+ (`self.CurrentTime`) (`GameplayStatics.GetWorldDeltaSeconds`))))
  (if (> _output_get (`self.DelayTime`))
    (set `self.CurrentTime` 0.0)
    (return true)
    (else
      (return false))))